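; Combat component for the third-person character that provides toggleable target lock-on.
; The target input sphere-traces forward from the camera for Pawns, stores the hit actor, and attaches a spawned lock-on widget actor above it.
; While locked, movement switches to controller-desired rotation and Tick aims control rotation at the target with a pitch offset.
; Pressing again clears the target, restores orient-to-movement and destroys the widget.
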(event `self.ReceiveBeginPlay`
  (bind _asbp_third_person_character (cast `/Game/ThirdPerson/Blueprints/BP_ThirdPersonCharacter` (`self.GetOwner`)))
  (set `self.Player BP` _asbp_third_person_character))

(event `EnhancedInput|/Game/ThirdPerson/Input/Actions/IA_Target`
  (params (ActionValue :type Boolean) (ElapsedSeconds :type "Float (double-precision)") (TriggeredSeconds :type "Float (double-precision)") (InputAction :type "InputAction Object Reference" :default "/Game/ThirdPerson/Input/Actions/IA_Target.IA_Target"))
  (bind _returnvalue (`Actor.GetTransform` (`self.TargetLockActor`)))
  (bind _transformcomponent (`PlayerCameraManager.TransformComponent` (`GameplayStatics.GetPlayerCameraManager` 0)))
  (bind _charactermovement (`Character.CharacterMovement` (`self.Player BP`)))
  (bind _charactermovement_2 (`Character.CharacterMovement` (`self.Player BP`)))
  (bind (_returnvalue_x _returnvalue_y _returnvalue_z) (`KismetMathLibrary.BreakVector` (`SceneComponent.K2_GetComponentLocation` _transformcomponent)))
  (bind _returnvalue_2 (`KismetMathLibrary.MakeVector` _returnvalue_x _returnvalue_y (+ _returnvalue_z 20.0)))
  (:`Started`
    (`self.TargetLockActor`
      (:`then`
        (set `self.TargetLockActor` null)
        (set `CharacterMovementComponent.bOrientRotationToMovement` true _charactermovement)
        (set `CharacterMovementComponent.bUseControllerDesiredRotation` false _charactermovement)
        (`Actor.K2_DestroyActor` (`self.Target Lock Widget`)))
      (:`else`
        (bind (_outhit _returnvalue_3) (`KismetSystemLibrary.SphereTraceSingleForObjects` :`Start` _returnvalue_2 :`End` (+ _returnvalue_2 (* (`KismetMathLibrary.GetForwardVector` (`SceneComponent.K2_GetComponentRotation` _transformcomponent)) 1000.0)) :`Radius` 150.0 :`ObjectTypes` (`|MakeArray` "ObjectTypeQuery3" :!type "EObjectTypeQuery Enum") :`DrawDebugType` "ForDuration" :`DrawTime` 2.0))
        (if _returnvalue_3
          (set `self.TargetLockActor` (`.HitActor` (`GameplayStatics.BreakHitResult` _outhit)))
          (set `CharacterMovementComponent.bOrientRotationToMovement` false _charactermovement_2)
          (set `CharacterMovementComponent.bUseControllerDesiredRotation` true _charactermovement_2)
          (bind _returnvalue_4 (`|SpawnActorFromClass` "/Game/Blueprints/BP_TargetLockWidget.BP_TargetLockWidget_C" (`KismetMathLibrary.MakeTransform` (`KismetMathLibrary.MakeVector` (.x (.location _returnvalue)) (.y (.location _returnvalue)) (+ (.z (.location _returnvalue)) 50.0)) (.rotation _returnvalue)) "AlwaysSpawn" "MultiplyWithRoot" null null))
          (bind _output_get (set `self.Target Lock Widget` _returnvalue_4))
          (`Actor.K2_AttachToActor` _output_get (`self.TargetLockActor`) "None" "KeepWorld" "SnapToTarget" "SnapToTarget" true))))))

(event `self.ReceiveTick`
  (params (DeltaSeconds :type "Float (single-precision)"))
  (bind _player_bp (`self.Player BP`))
  (bind _targetlockactor (`self.TargetLockActor`)
    (:`then`
      (bind (_returnvalue_roll _returnvalue_pitch _returnvalue_yaw) (`KismetMathLibrary.BreakRotator` (`KismetMathLibrary.FindLookAtRotation` (`Actor.K2_GetActorLocation` _player_bp) (`Actor.K2_GetActorLocation` _targetlockactor))))
      (`Controller.SetControlRotation` (`Pawn.GetController` _player_bp) (`KismetMathLibrary.MakeRotator` _returnvalue_roll (+ _returnvalue_pitch -20.0) _returnvalue_yaw)))
    (:`else`)))